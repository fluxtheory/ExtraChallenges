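; BP_RotatingCube is an actor that spins around its local yaw axis and periodically reverses direction.
; Tick calls the parent, then adds local rotation from RotationRate scaled by world delta seconds, keeping the speed frame-rate independent.
; It also accumulates CurrentTime and, on reaching TimeBetweenSwitch, negates RotationRate and resets the timer.
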(event `self.ReceiveBeginPlay`)

(event `self.ReceiveTick`
  (params (DeltaSeconds :type "Float (single-precision)"))
  (`parent.ReceiveTick` DeltaSeconds)
  ;[0 0 0] Rotate Actor. Multiplied by DeltaSeconds to make it frameRate independent.
  ; Google Frame Rate Dependency in games if that's new to you.
  (`self.K2_AddActorLocalRotation` (`KismetMathLibrary.MakeRotator` 0.0 0.0 (* (`GameplayStatics.GetWorldDeltaSeconds`) (`self.RotationRate`))))
  ;[0 0 0] Track Time between changing rotation direction
  (set `self.CurrentTime` (+ (`self.CurrentTime`) (`GameplayStatics.GetWorldDeltaSeconds`)))
  ;[0 0 0] If timer hits limit, switch rotation rate. Reset tracked time
  (if (>= (`self.CurrentTime`) (`self.TimeBetweenSwitch`))
    (set `self.RotationRate` (* (`self.RotationRate`) -1.0))
    (set `self.CurrentTime` 0.0)))

(fn `UserConstructionScript`)