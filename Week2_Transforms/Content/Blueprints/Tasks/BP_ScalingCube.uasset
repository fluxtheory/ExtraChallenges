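; BP_ScalingCube is a task actor that pulses in size, growing and shrinking in alternating phases.
; Each Tick calls the parent tick, noted as C++ code, then adds ScaleFactor to the actor's scale.
; An accumulated delta-time timer negates ScaleFactor whenever it reaches TimeBetweenSwitch.
; The scale step is not multiplied by delta time, so its speed depends on frame rate.
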(event `self.ReceiveTick`
  (params (DeltaSeconds :type "Float (single-precision)"))
  (`parent.ReceiveTick` DeltaSeconds) ; THIS IS CALLING C++ CODE.
  (`self.SetActorScale3D` (+ (`self.ScaleFactor`) (`self.GetActorScale3D`)))
  (set `self.CurrentTime` (+ (`GameplayStatics.GetWorldDeltaSeconds`) (`self.CurrentTime`)))
  (if (>= (`self.CurrentTime`) (`self.TimeBetweenSwitch`))
    (set `self.CurrentTime` 0.0)
    (set `self.ScaleFactor` (* (`self.ScaleFactor`) -1.0))))

(fn `UserConstructionScript`)